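; BP_StopZone is a trigger zone that shows an interaction prompt widget when the player's BP_Ship enters it.
; Box collision overlaps store the ship reference and toggle the world widget, which rotates every tick to face the camera.
; A Checkboat event creates the configured widget on screen if the stored ship is still overlapping the box.
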(event `self.Box Collision.OnComponentBeginOverlap`
  (params (OverlappedComponent :type "PrimitiveComponent Object Reference") (OtherActor :type "Actor Object Reference") (OtherComp :type "PrimitiveComponent Object Reference") (OtherBodyIndex :type Integer) (bFromSweep :type Boolean) (SweepResult :type "HitResult Structure (by ref)"))
  (bind _asbp_ship (cast `/Game/Ship/BP_Ship` OtherActor))
  (set `self.As BP Ship` _asbp_ship)
  (`SceneComponent.SetVisibility` (`self.Widget Interact`) true false))

(event `self.Box Collision.OnComponentEndOverlap`
  (params (OverlappedComponent :type "PrimitiveComponent Object Reference") (OtherActor :type "Actor Object Reference") (OtherComp :type "PrimitiveComponent Object Reference") (OtherBodyIndex :type Integer))
  (cast `/Game/Ship/BP_Ship` OtherActor)
  (`SceneComponent.SetVisibility` (`self.Widget Interact`) false false))

(event `Checkboat`
  (for _array_element (`PrimitiveComponent.GetOverlappingActors` (`self.Box Collision`) null)
    (if (== _array_element (`self.As BP Ship`))
      (`self.CreateSpecifiedWidget`))))

(event `CreateSpecifiedWidget`
  (bind _returnvalue (`|CreateWidget` (`self.Widget`)))
  (`UserWidget.AddToViewport` _returnvalue 0))

(event `self.ReceiveTick`
  (params (DeltaSeconds :type "Float (single-precision)"))
  (bind _widget_interact (`self.Widget Interact`))
  (`SceneComponent.K2_SetWorldRotation` _widget_interact (`KismetMathLibrary.FindLookAtRotation` (`SceneComponent.K2_GetComponentLocation` _widget_interact) (`SceneComponent.K2_GetComponentLocation` (`PlayerCameraManager.TransformComponent` (`GameplayStatics.GetPlayerCameraManager` 0)))) false false))

(fn `UserConstructionScript`)